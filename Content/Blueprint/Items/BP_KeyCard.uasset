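; BP_KeyCard is a pickup key card shown as a Paper2D sprite, in red, orange or blue.
; The construction script sets the sprite from the KeyCard enum, and a looping timer yaws the actor toward the player as a billboard.
; When BP_PlayerCharacter overlaps the box, it sets that colour's key flag on the player, notifies the player HUD and destroys itself.
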(event `self.ReceiveBeginPlay`
  (`KismetSystemLibrary.K2_SetTimerDelegate` (delegate `LookAtPlayer`) 0.1 true)
  (`self.LookAtPlayer`))

(event `LookAtPlayer`
  (bind (_returnvalue_roll _returnvalue_pitch _returnvalue_yaw) (`KismetMathLibrary.BreakRotator` (`KismetMathLibrary.FindLookAtRotation` (`self.K2_GetActorLocation`) (`self.K2_GetActorLocation` (`GameplayStatics.GetPlayerCharacter` 0)))))
  (`self.K2_SetActorRotation` (`KismetMathLibrary.MakeRotator` 0.0 0.0 _returnvalue_yaw)))

(event `self.Box.OnComponentBeginOverlap`
  (params (OverlappedComponent :type "PrimitiveComponent Object Reference") (OtherActor :type "Actor Object Reference") (OtherComp :type "PrimitiveComponent Object Reference") (OtherBodyIndex :type Integer) (bFromSweep :type Boolean) (SweepResult :type "HitResult Structure (by ref)"))
  (bind _playercharacterref (`self.PlayerCharacterRef`))
  (bind _playercharacterref_2 (`self.PlayerCharacterRef`))
  (bind _playercharacterref_3 (`self.PlayerCharacterRef`))
  (bind _asbp_player_character (cast `/Game/Blueprint/BP_PlayerCharacter` OtherActor))
  (set `self.PlayerCharacterRef` _asbp_player_character)
  (switch `/Game/Blueprint/Items/Enum_KeyCard` (`self.KeyCard`)
    (:`NewEnumerator0`
      (set `/Game/Blueprint/BP_PlayerCharacter.bRedKeyCard` true _playercharacterref)
      (`/Game/Blueprint/UI/WBI_PlayerHUD.FindRedKeyCard` (`/Game/Blueprint/BP_PlayerCharacter.PlayerHUD` _playercharacterref)))
    (:`NewEnumerator1`
      (set `/Game/Blueprint/BP_PlayerCharacter.bOrangeKeyCard` true _playercharacterref_3)
      (`/Game/Blueprint/UI/WBI_PlayerHUD.FindOrangeKeyCard` (`/Game/Blueprint/BP_PlayerCharacter.PlayerHUD` _playercharacterref_3)))
    (:`NewEnumerator2`
      (set `/Game/Blueprint/BP_PlayerCharacter.bBlueKeyCard` true _playercharacterref_2)
      (`/Game/Blueprint/UI/WBI_PlayerHUD.FindBlueKeyCard` (`/Game/Blueprint/BP_PlayerCharacter.PlayerHUD` _playercharacterref_2))))
  (`self.K2_DestroyActor`))

(fn `UserConstructionScript`
  (switch `/Game/Blueprint/Items/Enum_KeyCard` (`self.KeyCard`)
    (:`NewEnumerator0`
      (`PaperSpriteComponent.SetSprite` (`self.PaperSprite`) "/Game/RetroFPSAssets/RetroFPSAssets/Items/redkey_Sprite.redkey_Sprite"))
    (:`NewEnumerator1`
      (`PaperSpriteComponent.SetSprite` (`self.PaperSprite`) "/Game/RetroFPSAssets/RetroFPSAssets/Items/orangekey_Sprite.orangekey_Sprite"))
    (:`NewEnumerator2`
      (`PaperSpriteComponent.SetSprite` (`self.PaperSprite`) "/Game/RetroFPSAssets/RetroFPSAssets/Items/bluekey_Sprite.bluekey_Sprite"))))