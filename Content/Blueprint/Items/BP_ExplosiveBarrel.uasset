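; Explosive barrel item drawn as a Paper2D flipbook that explodes on taking any damage, hurting nearby pawns.
; A looping timer turns the actor's yaw toward the player, so the sprite works as a billboard without using Tick.
; Damage swaps in an enlarged explosion flipbook and applies BarrelDamage to each hit from a debug-drawn sphere trace for pawns.
; The actor destroys itself after a delay equal to the flipbook's length.
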(event `self.ReceiveBeginPlay`
  (`KismetSystemLibrary.K2_SetTimerDelegate` (delegate `LookAtPlayer`) 0.1 true)
  (`self.LookAtPlayer`))

(event `LookAtPlayer`
  (bind (_returnvalue_roll _returnvalue_pitch _returnvalue_yaw) (`KismetMathLibrary.BreakRotator` (`KismetMathLibrary.FindLookAtRotation` (`self.K2_GetActorLocation`) (`self.K2_GetActorLocation` (`GameplayStatics.GetPlayerCharacter` 0)))))
  (`self.K2_SetActorRotation` (`KismetMathLibrary.MakeRotator` 0.0 0.0 _returnvalue_yaw)))

(event `self.ReceiveAnyDamage`
  (params (Damage :type "Float (single-precision)") (DamageType :type "DamageType Object Reference") (InstigatedBy :type "Controller Object Reference") (DamageCauser :type "Actor Object Reference"))
  (bind _returnvalue (`self.K2_GetActorLocation`))
  (`PaperFlipbookComponent.SetFlipbook` (`self.PaperFlipbook`) "/Game/RetroFPSAssets/RetroFPSAssets/Projectiles/Rocket/FB_Explosion.FB_Explosion")
  (`SceneComponent.SetWorldScale3D` (`self.PaperFlipbook`) (10.0 10.0 10.0))
  (bind _outhits (`KismetSystemLibrary.SphereTraceMultiForObjects` :`Start` _returnvalue :`End` _returnvalue :`Radius` 450.0 :`ObjectTypes` (`|MakeArray` "ObjectTypeQuery3" :!type "EObjectTypeQuery Enum") :`DrawDebugType` "ForDuration"))
  (for _array_element _outhits
    (`GameplayStatics.ApplyDamage` (`.HitActor` (`GameplayStatics.BreakHitResult` _array_element)) (`self.BarrelDamage`)))
  (`KismetSystemLibrary.Delay` (`PaperFlipbookComponent.GetFlipbookLength` (`self.PaperFlipbook`)))
  (`self.K2_DestroyActor`))

(fn `UserConstructionScript`)