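; BP_Chainsaw is a chainsaw weapon that attacks continuously while shooting, using Paper2D flipbooks for its visuals.
; ShootWeapon passes through a DoOnce to start a fast looping timer, which calls FireWeapon and sets the attack flipbook on each tick.
; StopShooting clears that timer, restores the idle flipbook and resets the DoOnce, so repeated shoot calls cannot stack timers.
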(event `self.ShootWeapon`
  (`/Engine/EditorBlueprintResources/StandardMacros.DoOnce` false :!label _label
    (:`Completed`
      (bind _returnvalue (`KismetSystemLibrary.K2_SetTimerDelegate` (delegate `UseCahinsaw`) 0.15 true))
      (set `self.ChainsawEvent` _returnvalue))))

(event `ResetChainsaw`
  (goto _label :!via `Reset`))

(event `UseCahinsaw`
  (`self.FireWeapon`)
  (`PaperFlipbookComponent.SetFlipbook` (`self.WeaponFlipbook`) "/Game/RetroFPSAssets/RetroFPSAssets/Weapons/Chainsaw/FB_ChainAttack.FB_ChainAttack"))

(event `self.StopShooting`
  (`KismetSystemLibrary.K2_ClearAndInvalidateTimerHandle` (`self.ChainsawEvent`))
  (`PaperFlipbookComponent.SetFlipbook` (`self.WeaponFlipbook`) "/Game/RetroFPSAssets/RetroFPSAssets/Weapons/Chainsaw/FB_ChainIdle.FB_ChainIdle")
  (`self.ResetChainsaw`))

(fn `UserConstructionScript`
  (`parent.UserConstructionScript`))