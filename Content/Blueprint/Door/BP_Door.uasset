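; BP_Door is an interactable door actor that swings open and closed.
; An Interact event calls ToggleDoor, which picks OpenDoor or CloseDoor from the IsOpen flag.
; Each uses MoveComponentTo to ease the Door component between its closed rotation and a quarter turn over half a second, setting IsOpen afterwards.
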(event `/Game/Blueprint/BPI_InteractInterface.Interact`
  (`self.ToggleDoor`))

(event `ToggleDoor`
  (if (`self.bIsOpen`)
    (`self.CloseDoor`)
    (else
      (`self.OpenDoor`))))

(event `OpenDoor`
  (`KismetSystemLibrary.MoveComponentTo` (`self.Door`) (0.0 0.0 0.0) (struct :`Yaw` 90.0) true true 0.5)
  (set `self.bIsOpen` true))

(event `CloseDoor`
  (`KismetSystemLibrary.MoveComponentTo` (`self.Door`) (0.0 0.0 0.0) (struct) true true 0.5)
  (set `self.bIsOpen` false))

(fn `UserConstructionScript`)