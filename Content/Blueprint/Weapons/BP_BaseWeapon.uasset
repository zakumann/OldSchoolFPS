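; Base weapon Blueprint providing shared hitscan firing and ammo logic, with empty ShootWeapon and StopShooting events.
; FireWeapon line-traces forward from the LineTrace component, ignoring itself and the player, and applies WeaponDamage to the hit actor with debug drawing on.
; HasEnoughAmmo and DecreaseAmmo switch on AmmoType (bullet, shell, rocket, cell) to check or decrement counters stored on the cached player character, updating its HUD after each decrement.
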(event `self.ReceiveBeginPlay`
  (bind _asbp_player_character (cast `/Game/Blueprint/BP_PlayerCharacter` (`GameplayStatics.GetPlayerCharacter` 0)))
  (set `self.PlayerCharacterRef` _asbp_player_character))

(event `ShootWeapon`)

(event `StopShooting`)

(event `DecreaseAmmo`
  (bind _playercharacterref (`self.PlayerCharacterRef`))
  (bind _playercharacterref_2 (`self.PlayerCharacterRef`))
  (bind _playercharacterref_3 (`self.PlayerCharacterRef`))
  (bind _playercharacterref_4 (`self.PlayerCharacterRef`))
  (switch `/Game/Blueprint/Weapons/Enum_Ammo` (`self.AmmoType`)
    (:`NewEnumerator0`
      (`/Engine/EditorBlueprintResources/StandardMacros.DecrementInt` (`/Game/Blueprint/BP_PlayerCharacter.Bullet` _playercharacterref_2)
        (:`  `
          (`/Game/Blueprint/UI/WBI_PlayerHUD.UpdateBulletAmmo` (`/Game/Blueprint/BP_PlayerCharacter.PlayerHUD` _playercharacterref_2)))))
    (:`NewEnumerator1`
      (`/Engine/EditorBlueprintResources/StandardMacros.DecrementInt` (`/Game/Blueprint/BP_PlayerCharacter.Shell` _playercharacterref_3)
        (:`  `
          (`/Game/Blueprint/UI/WBI_PlayerHUD.UpdateShellAmmo` (`/Game/Blueprint/BP_PlayerCharacter.PlayerHUD` _playercharacterref_3)))))
    (:`NewEnumerator2`
      (`/Engine/EditorBlueprintResources/StandardMacros.DecrementInt` (`/Game/Blueprint/BP_PlayerCharacter.Rocket` _playercharacterref_4)
        (:`  `
          (`/Game/Blueprint/UI/WBI_PlayerHUD.UpdateRocketAmmo` (`/Game/Blueprint/BP_PlayerCharacter.PlayerHUD` _playercharacterref_4)))))
    (:`NewEnumerator3`
      (`/Engine/EditorBlueprintResources/StandardMacros.DecrementInt` (`/Game/Blueprint/BP_PlayerCharacter.Cell` _playercharacterref)
        (:`  `
          (`/Game/Blueprint/UI/WBI_PlayerHUD.UpdateCellAmmo` (`/Game/Blueprint/BP_PlayerCharacter.PlayerHUD` _playercharacterref)))))))

(fn `FireWeapon`
  (bind _returnvalue (`SceneComponent.K2_GetComponentLocation` (`self.LineTrace`)))
  (bind (_outhit _returnvalue_2) (`KismetSystemLibrary.LineTraceSingleForObjects` _returnvalue (+ _returnvalue (* (`KismetMathLibrary.GetForwardVector` (`SceneComponent.K2_GetComponentRotation` (`self.LineTrace`))) (`self.LineTraceDistance`))) (`|MakeArray` "ObjectTypeQuery1" "ObjectTypeQuery2" "ObjectTypeQuery3" :!type "EObjectTypeQuery Enum") false (`|MakeArray` self (`GameplayStatics.GetPlayerCharacter` 0) :!type "Actor Object Reference") "ForDuration"))
  (if _returnvalue_2
    (`GameplayStatics.ApplyDamage` (`.HitActor` (`GameplayStatics.BreakHitResult` _outhit)) (`self.WeaponDamage`))))

(fn `HasEnoughAmmo`
  (returns (hasAmmo :type Boolean))
  (switch `/Game/Blueprint/Weapons/Enum_Ammo` (`self.AmmoType`)
    (:`NewEnumerator0`
      ; Bullet
      (if (> (`/Game/Blueprint/BP_PlayerCharacter.Bullet` (`self.PlayerCharacterRef`)) 0)
        (return true)
        (else
          (return false))))
    (:`NewEnumerator1`
      ; Shell
      (if (> (`/Game/Blueprint/BP_PlayerCharacter.Shell` (`self.PlayerCharacterRef`)) 0)
        (return true)
        (else
          (return false))))
    (:`NewEnumerator2`
      ; Rocket
      (if (> (`/Game/Blueprint/BP_PlayerCharacter.Rocket` (`self.PlayerCharacterRef`)) 0)
        (return true)
        (else
          (return false))))
    (:`NewEnumerator3`
      ; Cell
      (if (> (`/Game/Blueprint/BP_PlayerCharacter.Cell` (`self.PlayerCharacterRef`)) 0)
        (return true)
        (else
          (return false))))))

(fn `UserConstructionScript`)