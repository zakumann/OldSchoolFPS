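; BP_BFG is a BFG weapon that fires a projectile using the player's Cell ammo.
; ShootWeapon requires more than 30 cells and uses a DoOnce gate to block overlapping shots.
; It plays the fire flipbook, waits for its length, then launches the projectile and restores the idle flipbook.
; It then deducts the ammo cost, updates the HUD and calls ResetShooting to reopen the gate.
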(event `self.ShootWeapon`
  (bind _playercharacterref (`self.PlayerCharacterRef`))
  (bind _weaponflipbook (`self.WeaponFlipbook`))
  (if (> (`/Game/Blueprint/BP_PlayerCharacter.Cell` (`self.PlayerCharacterRef`)) 30)
    (`/Engine/EditorBlueprintResources/StandardMacros.DoOnce` false :!label _label
      (:`Completed`
        (`PaperFlipbookComponent.SetFlipbook` _weaponflipbook "/Game/RetroFPSAssets/RetroFPSAssets/Weapons/BFG/FB_BFGFire.FB_BFGFire")
        (`KismetSystemLibrary.Delay` (`PaperFlipbookComponent.GetFlipbookLength` _weaponflipbook))
        (`self.FireProjectile`)
        (`PaperFlipbookComponent.SetFlipbook` (`self.WeaponFlipbook`) "/Game/RetroFPSAssets/RetroFPSAssets/Weapons/BFG/FB_BFGIdle.FB_BFGIdle")
        (set `/Game/Blueprint/BP_PlayerCharacter.Cell` (- (`/Game/Blueprint/BP_PlayerCharacter.Cell` _playercharacterref) 30) _playercharacterref)
        (`/Game/Blueprint/UI/WBI_PlayerHUD.UpdateCellAmmo` (`/Game/Blueprint/BP_PlayerCharacter.PlayerHUD` _playercharacterref))
        (`self.ResetShooting`)))))

(event `ResetShooting`
  (goto _label :!via `Reset`))

(fn `UserConstructionScript`
  (`parent.UserConstructionScript`))