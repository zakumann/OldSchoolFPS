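; BP_KeyCardDoor is an interactable door that only toggles if the player holds the key card matching its configured colour.
; On Interact it casts the player to BP_PlayerCharacter, checks the red, orange or blue card flag selected by the KeyCardDoor enum, then opens or closes.
; Opening and closing rotate the Door component with an eased MoveComponentTo.
; The construction script sets the door material from the same enum.
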(event `/Game/Blueprint/Interface/BPI_InteractInterface.Interact`
  (`self.ToggleDoor`))

(event `ToggleDoor`
  (bind _asbp_player_character (cast `/Game/Blueprint/BP_PlayerCharacter` (`GameplayStatics.GetPlayerCharacter` 0)))
  (set `self.As BP Player Character` _asbp_player_character)
  (switch `/Game/Blueprint/Items/Enum_KeyCard` (`self.KeyCardDoor`)
    (:`NewEnumerator0`
      (if (`/Game/Blueprint/BP_PlayerCharacter.bRedKeyCard` (`self.As BP Player Character`))
        (if (`self.bIsOpen`) :!label _label
          (`self.CloseDoor`)
          (else
            (`self.OpenDoor`)))))
    (:`NewEnumerator1`
      (if (`/Game/Blueprint/BP_PlayerCharacter.bOrangeKeyCard` (`self.As BP Player Character`))
        (goto _label)))
    (:`NewEnumerator2`
      (if (`/Game/Blueprint/BP_PlayerCharacter.bBlueKeyCard` (`self.As BP Player Character`))
        (goto _label)))))

(event `OpenDoor`
  (`KismetSystemLibrary.MoveComponentTo` (`self.Door`) (0.0 0.0 0.0) (struct :`Yaw` 90.0) true true 0.5)
  (set `self.bIsOpen` true))

(event `CloseDoor`
  (`KismetSystemLibrary.MoveComponentTo` (`self.Door`) (0.0 0.0 0.0) (struct) true true 0.5)
  (set `self.bIsOpen` false))

(fn `UserConstructionScript`
  (switch `/Game/Blueprint/Items/Enum_KeyCard` (`self.KeyCardDoor`)
    (:`NewEnumerator0`
      (`PrimitiveComponent.SetMaterial` (`self.Door`) 0 "/Game/RetroFPSAssets/RetroFPSAssets/Items/reddoor_Mat.reddoor_Mat"))
    (:`NewEnumerator1`
      (`PrimitiveComponent.SetMaterial` (`self.Door`) 0 "/Game/RetroFPSAssets/RetroFPSAssets/Items/Orangedoor_Mat.Orangedoor_Mat"))
    (:`NewEnumerator2`
      (`PrimitiveComponent.SetMaterial` (`self.Door`) 0 "/Game/RetroFPSAssets/RetroFPSAssets/Items/bluedoor_Mat.bluedoor_Mat"))))