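; BP_HealthPickup is a pickup that restores the player character's health when they overlap its box.
; A DoOnce gate guards the overlap, resetting if health is already full so the pickup stays available.
; Otherwise it adds HealthAmount clamped to MaxHealth, updates the player's HUD and destroys itself.
; A looping timer, rather than Tick, turns the pickup's yaw to face the player.
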(event `self.ReceiveBeginPlay`
  (`KismetSystemLibrary.K2_SetTimerDelegate` (delegate `LookAtPlayer`) 0.1 true)
  (`self.LookAtPlayer`))

(event `LookAtPlayer`
  (bind (_returnvalue_roll _returnvalue_pitch _returnvalue_yaw) (`KismetMathLibrary.BreakRotator` (`KismetMathLibrary.FindLookAtRotation` (`self.K2_GetActorLocation`) (`self.K2_GetActorLocation` (`GameplayStatics.GetPlayerCharacter` 0)))))
  (`self.K2_SetActorRotation` (`KismetMathLibrary.MakeRotator` 0.0 0.0 _returnvalue_yaw)))

(event `self.Box.OnComponentBeginOverlap`
  (params (OverlappedComponent :type "PrimitiveComponent Object Reference") (OtherActor :type "Actor Object Reference") (OtherComp :type "PrimitiveComponent Object Reference") (OtherBodyIndex :type Integer) (bFromSweep :type Boolean) (SweepResult :type "HitResult Structure (by ref)"))
  (bind _as_bp_player_character (`self.As BP Player Character`))
  (bind _asbp_player_character (cast `/Game/Blueprint/BP_PlayerCharacter` OtherActor))
  (bind _output_get (set `self.As BP Player Character` _asbp_player_character))
  (`/Engine/EditorBlueprintResources/StandardMacros.DoOnce` false :!label _label
    (:`Completed`
      (if (== (`/Game/Blueprint/BP_PlayerCharacter.Health` _as_bp_player_character) (`/Game/Blueprint/BP_PlayerCharacter.MaxHealth` _as_bp_player_character))
        (`self.ResetPickup`)
        (else
          (set `/Game/Blueprint/BP_PlayerCharacter.Health` (`KismetMathLibrary.FClamp` (+ (`/Game/Blueprint/BP_PlayerCharacter.Health` _output_get) (`self.HealthAmount`)) 0.0 (`/Game/Blueprint/BP_PlayerCharacter.MaxHealth` _output_get)) _output_get)
          (`/Game/Blueprint/UI/WBI_PlayerHUD.UpdatePlayerHealth` (`/Game/Blueprint/BP_PlayerCharacter.PlayerHUD` _output_get))
          (`self.K2_DestroyActor`))))))

(event `ResetPickup`
  (goto _label :!via `Reset`))

(fn `UserConstructionScript`)