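; Ammo pickup actor that gives the player bullets, shells, rockets or cells, with its sprite set from AmmoType in the construction script.
; A looping timer yaws it toward the player as a billboard.
; On box overlap with BP_PlayerCharacter, a DoOnce gate adds the clamped amount, updates the matching HUD counter and destroys the actor.
; If that ammo is already full, the gate resets so the pickup remains available.
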(event `self.ReceiveBeginPlay`
  (`KismetSystemLibrary.K2_SetTimerDelegate` (delegate `LookAtPlayer`) 0.1 true)
  (`self.LookAtPlayer`))

(event `LookAtPlayer`
  (bind (_returnvalue_roll _returnvalue_pitch _returnvalue_yaw) (`KismetMathLibrary.BreakRotator` (`KismetMathLibrary.FindLookAtRotation` (`self.K2_GetActorLocation`) (`self.K2_GetActorLocation` (`GameplayStatics.GetPlayerCharacter` 0)))))
  (`self.K2_SetActorRotation` (`KismetMathLibrary.MakeRotator` 0.0 0.0 _returnvalue_yaw)))

(event `self.Box.OnComponentBeginOverlap`
  (params (OverlappedComponent :type "PrimitiveComponent Object Reference") (OtherActor :type "Actor Object Reference") (OtherComp :type "PrimitiveComponent Object Reference") (OtherBodyIndex :type Integer) (bFromSweep :type Boolean) (SweepResult :type "HitResult Structure (by ref)"))
  (bind _as_bp_player_character (`self.As BP Player Character`))
  (bind _as_bp_player_character_2 (`self.As BP Player Character`))
  (bind _as_bp_player_character_3 (`self.As BP Player Character`))
  (bind _as_bp_player_character_4 (`self.As BP Player Character`))
  (bind _as_bp_player_character_5 (`self.As BP Player Character`))
  (bind _as_bp_player_character_6 (`self.As BP Player Character`))
  (bind _as_bp_player_character_7 (`self.As BP Player Character`))
  (bind _as_bp_player_character_8 (`self.As BP Player Character`))
  (bind _as_bp_player_character_9 (`self.As BP Player Character`))
  (bind _as_bp_player_character_10 (`self.As BP Player Character`))
  (bind _as_bp_player_character_11 (`self.As BP Player Character`))
  (bind _as_bp_player_character_12 (`self.As BP Player Character`))
  (bind _asbp_player_character (cast `/Game/Blueprint/BP_PlayerCharacter` OtherActor))
  (set `self.As BP Player Character` _asbp_player_character)
  (`/Engine/EditorBlueprintResources/StandardMacros.DoOnce` false :!label _label
    (:`Completed`
      (switch `/Game/Blueprint/Items/Enum_AmmoType` (`self.AmmoType`)
        (:`NewEnumerator0`
          ; Bullet
          (if (!= (`/Game/Blueprint/BP_PlayerCharacter.Bullet` _as_bp_player_character_7) (`/Game/Blueprint/BP_PlayerCharacter.MaxBullet` _as_bp_player_character_7))
            (set `/Game/Blueprint/BP_PlayerCharacter.Bullet` (`KismetMathLibrary.Clamp` (+ (`/Game/Blueprint/BP_PlayerCharacter.Bullet` _as_bp_player_character) (`self.AmmoToGive`)) 0 (`/Game/Blueprint/BP_PlayerCharacter.MaxBullet` _as_bp_player_character)) _as_bp_player_character_11)
            (`/Game/Blueprint/UI/WBI_PlayerHUD.UpdateBulletAmmo` (`/Game/Blueprint/BP_PlayerCharacter.PlayerHUD` _as_bp_player_character_11))
            (`self.K2_DestroyActor`)
            (else
              (`self.ResetPickUp`))))
        (:`NewEnumerator1`
          ; Shell
          (if (!= (`/Game/Blueprint/BP_PlayerCharacter.Shell` _as_bp_player_character_9) (`/Game/Blueprint/BP_PlayerCharacter.MaxShell` _as_bp_player_character_9))
            (set `/Game/Blueprint/BP_PlayerCharacter.Shell` (`KismetMathLibrary.Clamp` (+ (`/Game/Blueprint/BP_PlayerCharacter.Shell` _as_bp_player_character_8) (`self.AmmoToGive`)) 0 (`/Game/Blueprint/BP_PlayerCharacter.MaxShell` _as_bp_player_character_8)) _as_bp_player_character_2)
            (`/Game/Blueprint/UI/WBI_PlayerHUD.UpdateShellAmmo` (`/Game/Blueprint/BP_PlayerCharacter.PlayerHUD` _as_bp_player_character_2))
            (`self.K2_DestroyActor`)
            (else
              (`self.ResetPickUp`))))
        (:`NewEnumerator2`
          ; Rocket
          (if (!= (`/Game/Blueprint/BP_PlayerCharacter.Rocket` _as_bp_player_character_10) (`/Game/Blueprint/BP_PlayerCharacter.MaxRocket` _as_bp_player_character_10))
            (set `/Game/Blueprint/BP_PlayerCharacter.Rocket` (`KismetMathLibrary.Clamp` (+ (`/Game/Blueprint/BP_PlayerCharacter.Rocket` _as_bp_player_character_3) (`self.AmmoToGive`)) 0 (`/Game/Blueprint/BP_PlayerCharacter.MaxRocket` _as_bp_player_character_3)) _as_bp_player_character_4)
            (`/Game/Blueprint/UI/WBI_PlayerHUD.UpdateRocketAmmo` (`/Game/Blueprint/BP_PlayerCharacter.PlayerHUD` _as_bp_player_character_4))
            (`self.K2_DestroyActor`)
            (else
              (`self.ResetPickUp`))))
        (:`NewEnumerator3`
          ; Cell
          (if (!= (`/Game/Blueprint/BP_PlayerCharacter.Cell` _as_bp_player_character_12) (`/Game/Blueprint/BP_PlayerCharacter.MaxCell` _as_bp_player_character_12))
            (set `/Game/Blueprint/BP_PlayerCharacter.Cell` (`KismetMathLibrary.Clamp` (+ (`/Game/Blueprint/BP_PlayerCharacter.Cell` _as_bp_player_character_5) (`self.AmmoToGive`)) 0 (`/Game/Blueprint/BP_PlayerCharacter.MaxCell` _as_bp_player_character_5)) _as_bp_player_character_6)
            (`/Game/Blueprint/UI/WBI_PlayerHUD.UpdateCellAmmo` (`/Game/Blueprint/BP_PlayerCharacter.PlayerHUD` _as_bp_player_character_6))
            (`self.K2_DestroyActor`)
            (else
              (`self.ResetPickUp`))))))))

(event `ResetPickUp`
  (goto _label :!via `Reset`))

(fn `UserConstructionScript`
  (switch `/Game/Blueprint/Items/Enum_AmmoType` (`self.AmmoType`)
    (:`NewEnumerator0`
      (`PaperSpriteComponent.SetSprite` (`self.PaperSprite`) "/Game/RetroFPSAssets/RetroFPSAssets/Items/NormalAmmo_Sprite.NormalAmmo_Sprite"))
    (:`NewEnumerator1`
      (`PaperSpriteComponent.SetSprite` (`self.PaperSprite`) "/Game/RetroFPSAssets/RetroFPSAssets/Items/Shotgun_Sprite.Shotgun_Sprite"))
    (:`NewEnumerator2`
      (`PaperSpriteComponent.SetSprite` (`self.PaperSprite`) "/Game/RetroFPSAssets/RetroFPSAssets/Items/Rocket_Sprite.Rocket_Sprite"))
    (:`NewEnumerator3`
      (`PaperSpriteComponent.SetSprite` (`self.PaperSprite`) "/Game/RetroFPSAssets/RetroFPSAssets/Items/cellammo_Sprite.cellammo_Sprite"))))