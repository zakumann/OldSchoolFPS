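; Plasma gun weapon Blueprint that fires projectiles automatically from shoot until stop.
; ShootWeapon passes a DoOnce gate and starts a looping timer, whose FirePlasma event checks and decreases ammo, fires a projectile and sets the firing flipbook.
; Running out of ammo or calling StopShooting follows a shared path that clears the timer, restores the idle flipbook and resets the gate.
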(event `self.ShootWeapon`
  (`/Engine/EditorBlueprintResources/StandardMacros.DoOnce` false :!label _label
    (:`Completed`
      (bind _returnvalue (`KismetSystemLibrary.K2_SetTimerDelegate` (delegate `FirePlasma`) 0.15 true))
      (set `self.PlasmaEvent` _returnvalue))))

(event `ResetFire`
  (goto _label :!via `Reset`))

(event `FirePlasma`
  (bind _hasammo (`self.HasEnoughAmmo`))
  (if _hasammo
    (`self.DecreaseAmmo`)
    (`self.FireProjectile`)
    (`PaperFlipbookComponent.SetFlipbook` (`self.WeaponFlipbook`) "/Game/RetroFPSAssets/RetroFPSAssets/Weapons/PlasmaGun/FB_PlasmaFire.FB_PlasmaFire")
    (else
      (`KismetSystemLibrary.K2_ClearAndInvalidateTimerHandle` (`self.PlasmaEvent`) :!label _label_2)
      (`PaperFlipbookComponent.SetFlipbook` (`self.WeaponFlipbook`) "/Game/RetroFPSAssets/RetroFPSAssets/Weapons/PlasmaGun/FB_PlasmaIdle.FB_PlasmaIdle")
      (`self.ResetFire`))))

(event `self.StopShooting`
  (goto _label_2))

(fn `UserConstructionScript`
  (`parent.UserConstructionScript`))