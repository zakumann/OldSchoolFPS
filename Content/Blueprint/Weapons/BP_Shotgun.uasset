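; Shotgun weapon Blueprint that fires when it has enough ammo and no weapon swap is flagged.
; ShootWeapon passes a DoOnce gate, then decreases ammo, calls FireWeapon and switches the Paper2D flipbook to the fire animation.
; After a delay equal to that flipbook's length, it restores the idle flipbook and calls ResetFire to reopen the gate, so animation length sets the fire rate.
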(event `self.ShootWeapon`
  (bind _weaponflipbook (`self.WeaponFlipbook`))
  (if (not (`self.bWeaponSwap`))
    (bind _hasammo (`self.HasEnoughAmmo`))
    (if _hasammo
      (`/Engine/EditorBlueprintResources/StandardMacros.DoOnce` false :!label _label
        (:`Completed`
          (`self.DecreaseAmmo`)
          (`self.FireWeapon`)
          (`PaperFlipbookComponent.SetFlipbook` _weaponflipbook "/Game/RetroFPSAssets/RetroFPSAssets/Weapons/Shotgun/FB_ShotgunFire.FB_ShotgunFire")
          (`KismetSystemLibrary.Delay` (`PaperFlipbookComponent.GetFlipbookLength` _weaponflipbook))
          (`PaperFlipbookComponent.SetFlipbook` (`self.WeaponFlipbook`) "/Game/RetroFPSAssets/RetroFPSAssets/Weapons/Shotgun/FB_ShotgunIdle.FB_ShotgunIdle")
          (`self.ResetFire`))))))

(event `ResetFire`
  (goto _label :!via `Reset`))

(fn `UserConstructionScript`
  (`parent.UserConstructionScript`))