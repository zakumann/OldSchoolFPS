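; Base pickup actor that turns to face the player and notifies player actors that touch it.
; A looping timer updates the actor's yaw toward player character 0 instead of using Tick.
; Overlap on PickUpBox sends an OverlapPickupMessage to any actor implementing INT_Player, passing itself.
; GetHealthAmount returns zero here.
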(event `self.ReceiveBeginPlay`
  (`KismetSystemLibrary.K2_SetTimerDelegate` (delegate `LookAtPlayer`) 0.1 true)
  (`self.LookAtPlayer`))

(event `LookAtPlayer`
  (bind (_returnvalue_roll _returnvalue_pitch _returnvalue_yaw) (`KismetMathLibrary.BreakRotator` (`KismetMathLibrary.FindLookAtRotation` (`self.K2_GetActorLocation`) (`self.K2_GetActorLocation` (`GameplayStatics.GetPlayerCharacter` 0)))))
  (`self.K2_SetActorRotation` (`KismetMathLibrary.MakeRotator` 0.0 0.0 _returnvalue_yaw)))

(event `self.PickUpBox.OnComponentBeginOverlap`
  (params (OverlappedComponent :type "PrimitiveComponent Object Reference") (OtherActor :type "Actor Object Reference") (OtherComp :type "PrimitiveComponent Object Reference") (OtherBodyIndex :type Integer) (bFromSweep :type Boolean) (SweepResult :type "HitResult Structure (by ref)"))
  (if (`KismetSystemLibrary.DoesImplementInterface` OtherActor "/Game/Blueprint/Interface/INT_Player.INT_Player_C")
    (message `/Game/Blueprint/Interface/INT_Player.OverlapPickup` OtherActor self)))

(fn `GetHealthAmount`
  (returns (Health :type "Float (double-precision)"))
  (return 0.0))

(fn `UserConstructionScript`)