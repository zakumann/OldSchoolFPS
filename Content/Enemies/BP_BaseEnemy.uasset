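; Base enemy with Doom-style eight-directional Paper2D sprites, player sensing, and melee and projectile attacks.
; A fast looping timer sets Idle or Moving from velocity, turns toward a seen player, and picks flipbook and sprite rotation using dot products against the player direction.
; PawnSensing sets the sight flag and blackboard key, cleared by a retriggerable delay.
; SpawnProjectile fires BP_EnemyProjectile; MeleeAttack line-traces forward to damage the player.
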(event `LookAtPlayer`
  (bind _returnvalue (`KismetMathLibrary.Normal` (- (`self.K2_GetActorLocation` (`GameplayStatics.GetPlayerCharacter` 0)) (`self.K2_GetActorLocation`))))
  (`KismetSystemLibrary.K2_SetTimerDelegate` (delegate `LookAtPlayer`) 0.01 true :!label _label)
  (if (> (`KismetMathLibrary.VSize` (`MovementComponent.Velocity` (`self.CharacterMovement`))) 0.0)
    (set `self.EnemyState` "NewEnumerator1")
    (else
      (set `self.EnemyState` "NewEnumerator0")))
  (if (`self.bCanSeePlayer`)
    (`self.RotateTowardsPlayer`))
  (set `self.Degrees` (`KismetMathLibrary.DegAcos` (`KismetMathLibrary.Dot_VectorVector` (`self.GetActorForwardVector`) _returnvalue)))
  (if (< (`KismetMathLibrary.Dot_VectorVector` (`self.GetActorRightVector`) _returnvalue) 0.0)
    (`/Engine/EditorBlueprintResources/StandardMacros.CompareFloat` (`self.Degrees`) 180.0
      (:`>`
        ; Front
        (`SceneComponent.K2_SetRelativeRotation` (`self.PaperFlipbook`) (struct :`Yaw` -90.0) false false :!label _label_2)
        (`PaperFlipbookComponent.SetFlipbook` (`self.PaperFlipbook`) (`|GetArrayItem` (select `/Game/Enemies/Enum_EnemyState` (`self.EnemyState`) :`NewEnumerator0` (`self.flipbooksIdle`) :`NewEnumerator1` (`self.flipbooksMoving`) :`NewEnumerator2` (`self.flipbooksMeleeAttack`) :`NewEnumerator3` (`self.flipbooksRangedAttack`)))))
      (:`==`
        (goto _label_2))
      (:`<`
        (`/Engine/EditorBlueprintResources/StandardMacros.CompareFloat` (`self.Degrees`) 135.0
          (:`>`
            ; BackLeft
            (`SceneComponent.K2_SetRelativeRotation` (`self.PaperFlipbook`) (struct :`Yaw` 135.0) false false :!label _label_3)
            (`PaperFlipbookComponent.SetFlipbook` (`self.PaperFlipbook`) (`|GetArrayItem` (select `/Game/Enemies/Enum_EnemyState` (`self.EnemyState`) :`NewEnumerator0` (`self.flipbooksIdle`) :`NewEnumerator1` (`self.flipbooksMoving`) :`NewEnumerator2` (`self.flipbooksMeleeAttack`) :`NewEnumerator3` (`self.flipbooksRangedAttack`)) 3)))
          (:`==`
            (goto _label_3))
          (:`<`
            (`/Engine/EditorBlueprintResources/StandardMacros.CompareFloat` (`self.Degrees`) 90.0
              (:`>`
                ; Left
                (`SceneComponent.K2_SetRelativeRotation` (`self.PaperFlipbook`) (struct :`Yaw` -180.0) false false :!label _label_4)
                (`PaperFlipbookComponent.SetFlipbook` (`self.PaperFlipbook`) (`|GetArrayItem` (select `/Game/Enemies/Enum_EnemyState` (`self.EnemyState`) :`NewEnumerator0` (`self.flipbooksIdle`) :`NewEnumerator1` (`self.flipbooksMoving`) :`NewEnumerator2` (`self.flipbooksMeleeAttack`) :`NewEnumerator3` (`self.flipbooksRangedAttack`)) 2)))
              (:`==`
                (goto _label_4))
              (:`<`
                (`/Engine/EditorBlueprintResources/StandardMacros.CompareFloat` (`self.Degrees`) 45.0
                  (:`>`
                    _)
                  (:`==`
                    _)
                  (:`<`
                    (goto _label_2)))
                ; FrontRight
                (`SceneComponent.K2_SetRelativeRotation` (`self.PaperFlipbook`) (struct :`Yaw` -135.0) false false)
                (`PaperFlipbookComponent.SetFlipbook` (`self.PaperFlipbook`) (`|GetArrayItem` (select `/Game/Enemies/Enum_EnemyState` (`self.EnemyState`) :`NewEnumerator0` (`self.flipbooksIdle`) :`NewEnumerator1` (`self.flipbooksMoving`) :`NewEnumerator2` (`self.flipbooksMeleeAttack`) :`NewEnumerator3` (`self.flipbooksRangedAttack`)) 1))))))))
    (else
      (`/Engine/EditorBlueprintResources/StandardMacros.CompareFloat` (`self.Degrees`) 180.0
        (:`>`
          ; FrontLeft
          (`SceneComponent.K2_SetRelativeRotation` (`self.PaperFlipbook`) (struct :`Yaw` -45.0) false false :!label _label_5)
          (`PaperFlipbookComponent.SetFlipbook` (`self.PaperFlipbook`) (`|GetArrayItem` (select `/Game/Enemies/Enum_EnemyState` (`self.EnemyState`) :`NewEnumerator0` (`self.flipbooksIdle`) :`NewEnumerator1` (`self.flipbooksMoving`) :`NewEnumerator2` (`self.flipbooksMeleeAttack`) :`NewEnumerator3` (`self.flipbooksRangedAttack`)) 7)))
        (:`==`
          (goto _label_5))
        (:`<`
          (`/Engine/EditorBlueprintResources/StandardMacros.CompareFloat` (`self.Degrees`) 135.0
            (:`>`
              ; Back
              (`SceneComponent.K2_SetRelativeRotation` (`self.PaperFlipbook`) (struct :`Yaw` 90.0) false false :!label _label_6)
              (`PaperFlipbookComponent.SetFlipbook` (`self.PaperFlipbook`) (`|GetArrayItem` (select `/Game/Enemies/Enum_EnemyState` (`self.EnemyState`) :`NewEnumerator0` (`self.flipbooksIdle`) :`NewEnumerator1` (`self.flipbooksMoving`) :`NewEnumerator2` (`self.flipbooksMeleeAttack`) :`NewEnumerator3` (`self.flipbooksRangedAttack`)) 4)))
            (:`==`
              (goto _label_6))
            (:`<`
              (`/Engine/EditorBlueprintResources/StandardMacros.CompareFloat` (`self.Degrees`) 90.0
                (:`>`
                  ; BackRight
                  (`SceneComponent.K2_SetRelativeRotation` (`self.PaperFlipbook`) (struct :`Yaw` 45.0) false false :!label _label_7)
                  (`PaperFlipbookComponent.SetFlipbook` (`self.PaperFlipbook`) (`|GetArrayItem` (select `/Game/Enemies/Enum_EnemyState` (`self.EnemyState`) :`NewEnumerator0` (`self.flipbooksIdle`) :`NewEnumerator1` (`self.flipbooksMoving`) :`NewEnumerator2` (`self.flipbooksMeleeAttack`) :`NewEnumerator3` (`self.flipbooksRangedAttack`)) 5)))
                (:`==`
                  (goto _label_7))
                (:`<`
                  (`/Engine/EditorBlueprintResources/StandardMacros.CompareFloat` (`self.Degrees`) 45.0
                    (:`>`
                      _)
                    (:`==`
                      _)
                    (:`<`
                      (goto _label_5)))
                  ; Right
                  (`SceneComponent.K2_SetRelativeRotation` :`self` (`self.PaperFlipbook`))
                  (`PaperFlipbookComponent.SetFlipbook` (`self.PaperFlipbook`) (`|GetArrayItem` (select `/Game/Enemies/Enum_EnemyState` (`self.EnemyState`) :`NewEnumerator0` (`self.flipbooksIdle`) :`NewEnumerator1` (`self.flipbooksMoving`) :`NewEnumerator2` (`self.flipbooksMeleeAttack`) :`NewEnumerator3` (`self.flipbooksRangedAttack`)) 6)))))))))))

(event `self.ReceiveBeginPlay`
  (goto _label))

(event `RotateTowardsPlayer`
  ; RotateTowardPlayer
  (`self.K2_SetActorRotation` (`KismetMathLibrary.RInterpTo` (`self.K2_GetActorRotation`) (`KismetMathLibrary.FindLookAtRotation` (`self.K2_GetActorLocation`) (`self.K2_GetActorLocation` (`GameplayStatics.GetPlayerCharacter` 0))) (`GameplayStatics.GetWorldDeltaSeconds`) (`self.RotationSpeed`))))

(event `self.PawnSensing.OnSeePawn`
  (params (Pawn :type "Pawn Object Reference"))
  ; bSeePlayer?
  (cast `/Game/Blueprint/BP_PlayerCharacter` Pawn)
  (set `self.bCanSeePlayer` true)
  (`BlackboardComponent.SetValueAsBool` (`AIBlueprintHelperLibrary.GetBlackboard` null) "bCanSeePlayer" true)
  (`KismetSystemLibrary.RetriggerableDelay` 0.7)
  (set `self.bCanSeePlayer` false)
  (`BlackboardComponent.SetValueAsBool` (`AIBlueprintHelperLibrary.GetBlackboard` null) "bCanSeePlayer" false))

(event `SpawnProjectile`
  ; bSeePlayer?
  (`|SpawnActorFromClass` "/Game/Enemies/BP_EnemyProjectile.BP_EnemyProjectile_C" (`SceneComponent.K2_GetComponentToWorld` (`self.ProjectileSpawn`)) "Undefined" "MultiplyWithRoot" null null))

(event `MeleeAttack`
  (bind _returnvalue (`self.K2_GetActorLocation`))
  (bind _outhit (`KismetSystemLibrary.LineTraceSingleForObjects` _returnvalue (+ _returnvalue (* (`self.GetActorForwardVector`) 150.0)) (`|MakeArray` "ObjectTypeQuery3" :!type "EObjectTypeQuery Enum") false (`|MakeArray` self :!type "Actor Object Reference") "ForDuration"))
  (bind (_bblockinghit _binitialoverlap _time _distance _location _impactpoint _normal _impactnormal _physmat _hitactor) (`GameplayStatics.BreakHitResult` _outhit))
  (if (== _hitactor (`GameplayStatics.GetPlayerCharacter` 0))
    (`GameplayStatics.ApplyDamage` _hitactor (`self.EnemyDamage`))))

(fn `UserConstructionScript`)