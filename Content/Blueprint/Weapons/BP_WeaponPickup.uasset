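; BP_WeaponPickup is a world pickup that gives the player a weapon when touched.
; The construction script uses the Weapon enum to set the Paper2D sprite and matching weapon class, covering guns and a chainsaw.
; A looping timer, rather than Tick, yaws the sprite toward the player as a billboard.
; On sphere overlap with BP_PlayerCharacter, it passes the class to PickupWeapon and destroys itself.
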(event `self.ReceiveBeginPlay`
  (`KismetSystemLibrary.K2_SetTimerDelegate` (delegate `LookAtPlayer`) 0.05 true)
  (`self.LookAtPlayer`))

(event `LookAtPlayer`
  (bind (_returnvalue_roll _returnvalue_pitch _returnvalue_yaw) (`KismetMathLibrary.BreakRotator` (`KismetMathLibrary.FindLookAtRotation` (`self.K2_GetActorLocation`) (`self.K2_GetActorLocation` (`GameplayStatics.GetPlayerCharacter` 0)))))
  (`self.K2_SetActorRotation` (`KismetMathLibrary.MakeRotator` 0.0 0.0 _returnvalue_yaw)))

(event `self.ReceiveTick`
  (params (DeltaSeconds :type "Float (single-precision)")))

(event `self.Sphere.OnComponentBeginOverlap`
  (params (OverlappedComponent :type "PrimitiveComponent Object Reference") (OtherActor :type "Actor Object Reference") (OtherComp :type "PrimitiveComponent Object Reference") (OtherBodyIndex :type Integer) (bFromSweep :type Boolean) (SweepResult :type "HitResult Structure (by ref)"))
  (bind _asbp_player_character (cast `/Game/Blueprint/BP_PlayerCharacter` OtherActor))
  (`/Game/Blueprint/BP_PlayerCharacter.PickupWeapon` _asbp_player_character (`self.WeaponClass`))
  (`self.K2_DestroyActor`))

(fn `UserConstructionScript`
  (switch `/Game/Blueprint/Weapons/Enum_Weapon` (`self.Weapon`)
    (:`NewEnumerator0`
      (`PaperSpriteComponent.SetSprite` (`self.PaperSprite`) "/Game/RetroFPSAssets/RetroFPSAssets/Weapons/Shotgun/Sprite_Shotgun.Sprite_Shotgun")
      (set `self.WeaponClass` "/Game/Blueprint/Weapons/BP_Shotgun.BP_Shotgun_C"))
    (:`NewEnumerator1`
      (`PaperSpriteComponent.SetSprite` (`self.PaperSprite`) "/Game/RetroFPSAssets/RetroFPSAssets/Weapons/MiniGun/Sprite_Minigun.Sprite_Minigun")
      (set `self.WeaponClass` "/Game/Blueprint/Weapons/BP_MiniGun.BP_MiniGun_C"))
    (:`NewEnumerator2`
      (`PaperSpriteComponent.SetSprite` (`self.PaperSprite`) "/Game/RetroFPSAssets/RetroFPSAssets/Weapons/PlasmaGun/Sprite_Plasma.Sprite_Plasma")
      (set `self.WeaponClass` "/Game/Blueprint/Weapons/BP_PlasmaGun.BP_PlasmaGun_C"))
    (:`NewEnumerator3`
      (`PaperSpriteComponent.SetSprite` (`self.PaperSprite`) "/Game/RetroFPSAssets/RetroFPSAssets/Weapons/RPG/Sprite_RPG.Sprite_RPG")
      (set `self.WeaponClass` "/Game/Blueprint/Weapons/BP_RPG.BP_RPG_C"))
    (:`NewEnumerator4`
      (`PaperSpriteComponent.SetSprite` (`self.PaperSprite`) "/Game/RetroFPSAssets/RetroFPSAssets/Weapons/BFG/Sprite_BFG.Sprite_BFG")
      (set `self.WeaponClass` "/Game/Blueprint/Weapons/BP_BFG.BP_BFG_C"))
    (:`NewEnumerator5`
      (`PaperSpriteComponent.SetSprite` (`self.PaperSprite`) "/Game/RetroFPSAssets/RetroFPSAssets/Weapons/Chainsaw/Sprite_Chainsaw.Sprite_Chainsaw")
      (set `self.WeaponClass` "/Game/Blueprint/Weapons/BP_Chainsaw.BP_Chainsaw_C"))))